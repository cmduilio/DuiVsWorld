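; BP_GridManager is an actor that lays out a rectangular grid of tile instances sized by SizeX and SizeY.
; Its construction script runs nested loops over rows and columns, adding one instance to the Tile component at fixed 100-unit spacing along X and Y.
; Using mesh instances avoids a separate actor per tile.
; The event graph holds only disabled placeholder events, so it has no gameplay logic.
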(event EventBeginPlay)

(event Collision|EventActorBeginOverlap
  (params (OtherActor :type Actor%20Object%20Reference)))

(event EventTick
  (params (DeltaSeconds :type Float%20%28single-precision%29)))

(fn ConstructionScript
  (for _index (range 0 (- (Variables|Default|GetSizeY) 1))
    (for _index_2 (range 0 (- (Variables|Default|GetSizeX) 1))
      (Components|InstancedStaticMesh|AddInstance (Variables|Default|GetTile) (Math|Transform|MakeTransform (Math|Vector|MakeVector (Math|Conversions|ToFloat(Integer) (* _index_2 100)) (Math|Conversions|ToFloat(Integer) (* _index 100)) 0.0) "0, 0, 0" "1,1,1")))))